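; Player pawn for BananaCollector, moved by forward and right axis input while its cube mesh bobs and spins.
; Axis events add speed-scaled movement input, which Tick consumes and applies as a swept local offset.
; Tick also runs SquashAndStretch, which only moves the cube up and down between world Z limits without scaling it, and Rotate, which yaws it at a constant rate.
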(event `InputAxis|MoveForward`
  (params (AxisValue :type "Float (single-precision)"))
  (`self.AddMovementInput` (`self.GetActorForwardVector`) (* AxisValue (`self.MaxSpeed`))))

(event `InputAxis|MoveRight`
  (params (AxisValue :type "Float (single-precision)"))
  (`self.AddMovementInput` (`self.GetActorRightVector`) (* AxisValue (`self.MaxSpeed`))))

(event `self.ReceiveTick`
  (params (DeltaSeconds :type "Float (single-precision)"))
  (`|ExecutionSequence`
    (:`then_0`
      (bind _returnvalue (`self.ConsumeMovementInputVector`))
      (`self.K2_AddActorLocalOffset` (* _returnvalue DeltaSeconds) true))
    (:`then_1`
      (`self.Squash and Stretch` DeltaSeconds))
    (:`then_2`
      (`self.Rotate` DeltaSeconds))))

(fn `Rotate`
  (params (`Delta Time` :type "Float (double-precision)"))
  (`SceneComponent.K2_AddLocalRotation` (`self.Cube`) (`KismetMathLibrary.MakeRotator` 0.0 0.0 (* `Delta Time` (`self.Spin Speed`))) false false))

(fn `Squash and Stretch`
  (params (`Delta Time` :type "Float (double-precision)"))
  (bind _squash___stretch_is_moving_up (`self.Squash & Stretch Is Moving Up`))
  (bind (_squash___stretch_range_x _squash___stretch_range_y) (`KismetMathLibrary.BreakVector` (`self.Squash & Stretch Range`)))
  (bind _cube (`self.Cube`))
  (bind (_returnvalue_x _returnvalue_y _returnvalue_z) (`KismetMathLibrary.BreakVector` (`SceneComponent.K2_GetComponentLocation` _cube)))
  (bind _returnvalue (* (`self.Squash & Stretch Speed`) `Delta Time`))
  (if _squash___stretch_is_moving_up
    (if (< _returnvalue_z _squash___stretch_range_x)
      (`SceneComponent.K2_AddLocalOffset` _cube (`KismetMathLibrary.MakeVector` 0.0 0.0 _returnvalue) false false)
      (else
        (set `self.Squash & Stretch Is Moving Up` (not _squash___stretch_is_moving_up) :!label _label)))
    (elif (> _returnvalue_z _squash___stretch_range_y)
      (`SceneComponent.K2_AddLocalOffset` _cube (`KismetMathLibrary.MakeVector` 0.0 0.0 (* _returnvalue -1.0)) false false)
      (else
        (goto _label)))))

(fn `UserConstructionScript`)